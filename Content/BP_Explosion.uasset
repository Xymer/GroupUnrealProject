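; BP_Explosion is an explosion actor that damages an actor overlapping its radius collider, then destroys itself.
; The collider's begin-overlap event sends ExplosionDamage to the other actor through an ApplyDamage message, with no radial query or falloff.
; It then draws a debug sphere matching the collider radius and spawns a particle effect at its location.
; Debug strings, including the overlapped actor's name, are printed along the way.
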(event `self.ActionRadiusCollider.OnComponentBeginOverlap`
  (params (OverlappedComponent :type "PrimitiveComponent Object Reference") (OtherActor :type "Actor Object Reference") (OtherComp :type "PrimitiveComponent Object Reference") (OtherBodyIndex :type Integer) (bFromSweep :type Boolean) (SweepResult :type "HitResult Structure (by ref)"))
  (bind _returnvalue (`self.K2_GetActorLocation` self))
  (`KismetSystemLibrary.PrintString` (`KismetSystemLibrary.GetDisplayName` OtherActor))
  (message `DamagableInterface.ApplyDamage` OtherActor (`self.ExplosionDamage`))
  (`KismetSystemLibrary.DrawDebugSphere` _returnvalue (`SphereComponent.SphereRadius` (`self.ActionRadiusCollider`)) 12 (struct :`R` 1.0 :`G` 1.0 :`B` 1.0 :`A` 1.0) (`self.DebugDuration`))
  (`GameplayStatics.SpawnEmitterAtLocation` (`self.ActionParticleEffect`) _returnvalue)
  (`self.K2_DestroyActor`)
  (`KismetSystemLibrary.PrintString` "ass"))

(fn `UserConstructionScript`)