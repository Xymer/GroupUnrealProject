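; BP_CharacterTest_DropWeapon is a functional test that checks whether a character can drop its weapon.
; On StartTest it has the Character pick up the test Weapon if it holds none, then immediately calls DropWeapon.
; It finishes as Succeeded if CurrentWeapon is then empty, otherwise as Failed.
; The timer variables are vestigial, so the check runs without any delay.
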(event `InputAxis|Fire`
  (params (AxisValue :type "Float (single-precision)")))

(event `self.ReceiveTick`
  (params (DeltaSeconds :type "Float (single-precision)")))

(event `self.ReceiveStartTest`
  (if (not (!= (`GroupUnrealProjectCharacter.CurrentWeapon` (`self.Character`)) null))
    (`GroupUnrealProjectCharacter.PickupWeapon` (`self.Character`) (`self.Weapon`)))
  (bind _output_get (set `self.TimerCurrent` (`self.TimerCurrent`)))
  (if true
    (`GroupUnrealProjectCharacter.DropWeapon` (`self.Character`))
    (if (== (`GroupUnrealProjectCharacter.CurrentWeapon` (`self.Character`)) null)
      (`self.FinishTest` "Succeeded" "Character dropped the weapon")
      (else
        (`self.FinishTest` "Failed" "Character still has a weapon")))))

(fn `UserConstructionScript`)