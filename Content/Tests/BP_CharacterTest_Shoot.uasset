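; Functional test that checks whether a character can fire a weapon.
; On start, a character with no current weapon picks up the test weapon and fails if its MagazineComponent has no ammo; an already armed character skips that check.
; It clears reloading, simulates a held fire input, calls OnFire directly, then immediately passes or fails on the weapon's HasFired flag.
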(event `self.ReceiveTick`
  (params (DeltaSeconds :type "Float (single-precision)")))

(event `self.ReceivePrepareTest`)

(event `self.ReceiveStartTest`
  (if (== (`GroupUnrealProjectCharacter.CurrentWeapon` (`self.Character`)) null)
    (`GroupUnrealProjectCharacter.PickupWeapon` (`self.Character`) (`self.Weapon`))
    (if (< 0 (`MagazineComponent.CurrentMagazineAmmoCount` (`self.GetComponentByClass` (`GroupUnrealProjectCharacter.CurrentWeapon` (`self.Character`)) "/Script/GroupUnrealProject.MagazineComponent")))
      (set `WeaponBase.bIsReloading` false (`GroupUnrealProjectCharacter.CurrentWeapon` (`self.Character`)) :!label _label)
      (bind _output_get (set `GroupUnrealProjectCharacter.FiringAxisValue` 1.0 (`self.Character`)))
      (set `GroupUnrealProjectCharacter.bIsFiring` (> _output_get 0.0) (`self.Character`))
      (`GroupUnrealProjectCharacter.OnFire` (`self.Character`))
      (if (`WeaponBase.bHasFired` (`GroupUnrealProjectCharacter.CurrentWeapon` (`self.Character`)))
        (`self.FinishTest` "Succeeded" "Weapon successfully fired.")
        (else
          (`self.FinishTest` "Failed" "Weapon did not fire.")))
      (else
        (`self.FinishTest` "Failed" "Did not have any ammo to fire.")))
    (else
      (goto _label))))

(fn `UserConstructionScript`)