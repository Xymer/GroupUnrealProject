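; Functional test that checks a character's ZoomIn narrows its camera field of view.
; On test start it can give the character a test weapon depending on its current one, then records the FOV and calls ZoomIn.
; It passes if the FOV is lower immediately afterwards, with no explicit failure branch.
; An unconnected debug chain that prints FOV around a zoom never runs.
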(event `self.ReceiveStartTest`
  (bind _character (`self.Character`))
  (bind _fieldofview (`CameraComponent.FieldOfView` (`self.GetComponentByClass` _character "/Script/Engine.CameraComponent")))
  (if (== (`GroupUnrealProjectCharacter.CurrentWeapon` (`self.Character`)) null)
    (`GroupUnrealProjectCharacter.PickupWeapon` _character (`self.Weapon`)))
  (bind _output_get (set `self.StartZoom` _fieldofview))
  (`GroupUnrealProjectCharacter.ZoomIn` (`self.Character`))
  (if (> _output_get _fieldofview)
    (`self.FinishTest` "Succeeded" "Successfully zoomed in.")))

(event `self.ReceiveTick`
  (params (DeltaSeconds :type "Float (single-precision)")))

(fn `UserConstructionScript`)