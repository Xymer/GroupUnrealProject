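; A functional test that checks whether a character's ChangeBullets action changes the current bullet on its equipped weapon.
; On test start it gives the character a weapon through PickupWeapon if its current weapon matches the check, then records the BulletComponent's CurrentBullet.
; It calls ChangeBullets and passes if CurrentBullet differs afterward, otherwise fails.
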(event `self.ReceiveStartTest`
  (bind _currentbullet (`BulletComponent.CurrentBullet` (`self.GetComponentByClass` (`GroupUnrealProjectCharacter.CurrentWeapon` (`self.Character`)) "/Script/GroupUnrealProject.BulletComponent")))
  (if (== (`GroupUnrealProjectCharacter.CurrentWeapon` (`self.Character`)) null)
    (`GroupUnrealProjectCharacter.PickupWeapon` (`self.Character`) (`self.Weapon`)))
  (bind _output_get (set `self.PreviousBullets` _currentbullet))
  (`GroupUnrealProjectCharacter.ChangeBullets` (`self.Character`))
  (if (!= _output_get _currentbullet)
    (`self.FinishTest` "Succeeded" "Changed bullets.")
    (else
      (`self.FinishTest` "Failed" "Failed to change bullets."))))

(fn `UserConstructionScript`)