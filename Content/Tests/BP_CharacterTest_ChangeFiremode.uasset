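; Functional test that verifies a character's weapon can switch fire mode.
; On test start it compares the character's current weapon and conditionally has the character pick up the test weapon.
; It records the weapon's fire mode, calls the switch, and finishes as succeeded if the mode differs or failed if it remains the same.
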(event `self.ReceiveStartTest`
  (bind _currentfiremode (`WeaponBase.CurrentFireMode` (`self.Weapon`)))
  (if (== (`GroupUnrealProjectCharacter.CurrentWeapon` (`self.Character`)) null)
    (`GroupUnrealProjectCharacter.PickupWeapon` (`self.Character`) (`self.Weapon`)))
  (set `self.OriginalFireMode` _currentfiremode)
  (`WeaponBase.SwitchFireMode` (`self.Weapon`))
  (if (!= (`self.OriginalFireMode`) _currentfiremode)
    (`self.FinishTest` "Succeeded" "Successfully changed firemode.")
    (else
      (`self.FinishTest` "Failed" "Firemode remains the same."))))

(fn `UserConstructionScript`)