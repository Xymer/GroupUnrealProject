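; Functional test that checks a character's weapon reload.
; On start, it has the Character pick up the Weapon if its current-weapon check passes, deducts from the weapon's ammo reserve, and records the MagazineComponent's ammo count.
; It then calls reload and immediately compares counts, succeeding when magazine ammo is equal or higher, so an unchanged magazine also passes despite the failure message expecting an increase.
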(event `self.ReceiveStartTest`
  (if (== (`GroupUnrealProjectCharacter.CurrentWeapon` (`self.Character`)) null)
    (`GroupUnrealProjectCharacter.PickupWeapon` (`self.Character`) (`self.Weapon`)))
  (`WeaponBase.DeductFromAmmoReserve` (`self.Weapon`) 1)
  (set `self.AmmoBeforeReload` (`MagazineComponent.CurrentMagazineAmmoCount` (`self.GetComponentByClass` (`self.Weapon`) "/Script/GroupUnrealProject.MagazineComponent")))
  (`GroupUnrealProjectCharacter.ReloadCurrentWeapon` (`self.Character`))
  (if (<= (`self.AmmoBeforeReload`) (`MagazineComponent.CurrentMagazineAmmoCount` (`self.GetComponentByClass` (`self.Weapon`) "/Script/GroupUnrealProject.MagazineComponent")))
    (`self.FinishTest` "Succeeded" "Successfully reloaded.")
    (else
      (`self.FinishTest` "Failed" "Reload failed did not increase the ammo in the magazine."))))

(fn `UserConstructionScript`)