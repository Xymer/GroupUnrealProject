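; BP_CharacterTest_AddAmmo is a functional test for adding reserve ammo to a character's weapon.
; On StartTest, if the CurrentWeapon check passes, the Character picks up Weapon and one round is added to its reserve.
; It compares the MagazineComponent's SelectedAmmoReserve before and after, finishing when the value is equal or higher, so an unchanged reserve also finishes.
; No branch reports failure, and the finish uses the Default result.
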(event `self.ReceiveStartTest`
  (bind _weapon (`self.Weapon`))
  (bind _selectedammoreserve (`MagazineComponent.SelectedAmmoReserve` (`self.GetComponentByClass` _weapon "/Script/GroupUnrealProject.MagazineComponent")))
  (if (== (`GroupUnrealProjectCharacter.CurrentWeapon` (`self.Character`)) null)
    (`GroupUnrealProjectCharacter.PickupWeapon` (`self.Character`) _weapon)
    (set `self.AmmoBeforeAdding` _selectedammoreserve)
    (`WeaponBase.AddToAmmoReserve` (`self.Weapon`) 1)
    (if (<= (`self.AmmoBeforeAdding`) _selectedammoreserve)
      (`self.FinishTest` "Default" "Ammo Successfully added."))))

(fn `UserConstructionScript`)