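; Functional test that verifies a character can change the magazine of its current weapon.
; On StartTest it has the character pick up a test weapon if its current weapon check passes, then records the weapon's MagazineComponent CurrentMagazine.
; It calls ChangeMagazine and succeeds if the current magazine differs afterward, otherwise it fails.
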(event `self.ReceiveStartTest`
  (bind _currentmagazine (`MagazineComponent.CurrentMagazine` (`self.GetComponentByClass` (`GroupUnrealProjectCharacter.CurrentWeapon` (`self.Character`)) "/Script/GroupUnrealProject.MagazineComponent")))
  (if (== (`GroupUnrealProjectCharacter.CurrentWeapon` (`self.Character`)) null)
    (`GroupUnrealProjectCharacter.PickupWeapon` (`self.Character`) (`self.Weapon`)))
  (bind _output_get (set `self.Previous Magazine` _currentmagazine))
  (`GroupUnrealProjectCharacter.ChangeMagazine` (`self.Character`))
  (if (!= _output_get _currentmagazine)
    (`self.FinishTest` "Succeeded" "Changed magazine.")
    (else
      (`self.FinishTest` "Failed" "Failed to change magazine."))))

(fn `UserConstructionScript`)